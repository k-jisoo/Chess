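; BP_ChessMap is a clickable chess board square that acts as a move destination for the selected piece.
; On BeginPlay it parses its grid X and Y from the first two characters of its display name.
; Clicking its plane registers it in BP_PlayerState, then runs KillProcess and Move on any selected piece with that position.
; It then clears the selection and sets every square's plane to the hidden material.
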(event OnClicked(Plane)
  (params (TouchedComponent :type Primitive%20Component%20Object%20Reference) (ButtonPressed :type Key%20Structure :default "None"))
  (bind _asbp_player_state (Utilities|Casting|CastToBP_PlayerState (Game|GetPlayerState 0)))
  (bind _output_get (Variables|/Game/Chess/BluePrints/BP_PlayerState.BP_PlayerState_C|SetSelectedMap _asbp_player_state self))
  (Utilities|IsValid (Variables|/Game/Chess/BluePrints/BP_PlayerState.BP_PlayerState_C|GetSelectedActor _asbp_player_state)
    (:Is%20Valid
      (Default|KillProcess (Variables|/Game/Chess/BluePrints/BP_PlayerState.BP_PlayerState_C|GetSelectedActor _asbp_player_state) (Variables|BP_ChessMap_C|GetPosX _output_get) (Variables|BP_ChessMap_C|GetPosY _output_get) (Variables|/Game/Chess/BluePrints/BP_PlayerState.BP_PlayerState_C|GetWholePieces _asbp_player_state))
      (Default|Move (Variables|/Game/Chess/BluePrints/BP_PlayerState.BP_PlayerState_C|GetSelectedActor _asbp_player_state) (Variables|BP_ChessMap_C|GetPosX _output_get) (Variables|BP_ChessMap_C|GetPosY _output_get))
      (Variables|/Game/Chess/BluePrints/BP_PlayerState.BP_PlayerState_C|SetSelectedActor _asbp_player_state 0)
      (Variables|/Game/Chess/BluePrints/BP_PlayerState.BP_PlayerState_C|SetSelectedMap _asbp_player_state 0)
      (for _array_element (Variables|/Game/Chess/BluePrints/BP_PlayerState.BP_PlayerState_C|GetChessMap _asbp_player_state)
        (Rendering|Material|SetMaterial (Variables|BP_ChessMap_C|GetPlane _array_element) 0 "/Game/Chess/Material/MI_PlaneHidden.MI_PlaneHidden")))))

(event EventBeginPlay
  (bind _self self)
  (bind _returnvalue (Utilities|GetDisplayName _self))
  (Variables|Default|SetPosX (Math|Conversions|ToInteger(Byte) (Utilities|String|GetSubstring _returnvalue 0)))
  (Variables|Default|SetPosY (Math|Conversions|ToInteger(Byte) (Utilities|String|GetSubstring _returnvalue 1))))

(fn ConstructionScript)